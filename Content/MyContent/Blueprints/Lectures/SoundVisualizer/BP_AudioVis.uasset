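; BP_AudioVis is a sound visualizer lecture actor that shows two widget components while the VR player stands inside its trigger box.
; On BeginPlay it tints the Tekst and Slika elements of the W_AudioVis widget, then hides both components.
; Box overlap begin and end events toggle their visibility, reacting only to actors whose class is exactly VRPawn.
; If the W_AudioVis cast fails, the initial hide is skipped.
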(event OnComponentBeginOverlap(Box)
  (params (OverlappedComponent :type Primitive%20Component%20Object%20Reference) (OtherActor :type Actor%20Object%20Reference) (OtherComp :type Primitive%20Component%20Object%20Reference) (OtherBodyIndex :type Integer) (bFromSweep :type Boolean) (SweepResult :type Hit%20Result%20Structure%20%28by%20ref%29))
  (if (== (Utilities|GetClass OtherActor) "/Game/VRTemplate/Blueprints/VRPawn.VRPawn_C")
    (Rendering|SetVisibility (Variables|Default|GetWidget) true true)))

(event OnComponentEndOverlap(Box)
  (params (OverlappedComponent :type Primitive%20Component%20Object%20Reference) (OtherActor :type Actor%20Object%20Reference) (OtherComp :type Primitive%20Component%20Object%20Reference) (OtherBodyIndex :type Integer))
  (if (== (Utilities|GetClass OtherActor) "/Game/VRTemplate/Blueprints/VRPawn.VRPawn_C")
    (Rendering|SetVisibility (Variables|Default|GetWidget) false false)))

(event EventBeginPlay
  (bind _asw_audio_vis (Utilities|Casting|CastToW_AudioVis (UserInterface|GetWidget (Variables|Default|GetWidget))))
  (Class|Button|SetBackgroundColor (Variables|/Game/MyContent/Blueprints/Lectures/SoundVisualizer/W_AudioVis.W_AudioVis_C|GetTekst _asw_audio_vis) (Utilities|Struct|MakeLinearColor 0.83 0.0 0.17 0.88))
  (Class|Button|SetBackgroundColor (Variables|/Game/MyContent/Blueprints/Lectures/SoundVisualizer/W_AudioVis.W_AudioVis_C|GetSlika _asw_audio_vis) (Utilities|Struct|MakeLinearColor 0.2 0.0 0.01 0.8))
  (Rendering|SetVisibility (Variables|Default|GetWidget) false false))

(event Collision|EventActorBeginOverlap
  (params (OtherActor :type Actor%20Object%20Reference)))

(event EventTick
  (params (DeltaSeconds :type Float%20%28single-precision%29)))

(fn ConstructionScript)