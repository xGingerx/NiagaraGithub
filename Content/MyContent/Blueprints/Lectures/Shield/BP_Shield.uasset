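; BP_Shield is a shield actor that reacts to hits with sound, Niagara particles and an animated material ripple.
; On hit, it writes the impact point to a dynamic material, and a timeline drives the ripple radius.
; Each hit raises the material's distortion until it passes a threshold and resets.
; That material parameter doubles as shield state, feeding the W_Shield widget's number and shrinking bar during timeline updates.
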(event OnComponentHit(StaticMesh)
  (params (HitComponent :type Primitive%20Component%20Object%20Reference) (OtherActor :type Actor%20Object%20Reference) (OtherComp :type Primitive%20Component%20Object%20Reference) (NormalImpulse :type Vector :default "0, 0, 0") (Hit :type Hit%20Result%20Structure%20%28by%20ref%29))
  ;[1 1 1] Spawnaj manji krug na mjestu udarca
  (Audio|PlaySound2D "/Game/MyContent/SoundEffects/shieldimpact.shieldimpact" 1.0 1.0 0.0 0 0)
  (bind _returnvalue (Rendering|Material|CreateDynamicMaterialInstance (Variables|Default|GetStaticMesh) 0 0 "None" :!class /Script/Engine.PrimitiveComponent))
  (Rendering|Material|SetVectorParameterValue _returnvalue "Pos" (Math|Conversions|ToLinearColor(Vector) (.impactpoint Hit)) :!class /Script/Engine.MaterialInstanceDynamic)
  ;[1 1 1] Promijeni distorciju materijala nakon svakog udarca
  (bind _returnvalue_2 (Rendering|Material|GetScalarParameterValue _returnvalue "DistortionIntes" :!class /Script/Engine.MaterialInstanceDynamic))
  (if (<= _returnvalue_2 6.0)
    (Rendering|Material|SetScalarParameterValue _returnvalue "DistortionIntes" (+ _returnvalue_2 (Variables|Default|GetAddDistortion)) :!class /Script/Engine.MaterialInstanceDynamic)
    (else
      (Rendering|Material|SetScalarParameterValue _returnvalue "DistortionIntes" 0.3 :!class /Script/Engine.MaterialInstanceDynamic)))
  ;[1 1 1] Spawn niagara efekt i animiraj materijal da pokaze manji krug pri udarcu o shield
  (Niagara|SpawnSystematLocation "/Game/MyContent/NiagaraVFX/Shield/NF_ExplodeParticle.NF_ExplodeParticle" (.impactpoint Hit) (Math|Rotator|MakeRotfromX (.normal Hit)))
  (bind _newtrack_0 (Timeline|Animate PlayFromStart)
    (:Update
      (Rendering|Material|SetScalarParameterValue _returnvalue "Radius" (* _newtrack_0 2e+02) :!class /Script/Engine.MaterialInstanceDynamic)
      (bind _asw_shield (Utilities|Casting|CastToW_Shield (UserInterface|GetWidget (Variables|Default|GetWidget))))
      (bind _returnvalue_3 (Rendering|Material|GetScalarParameterValue _returnvalue "DistortionIntes" :!class /Script/Engine.MaterialInstanceDynamic))
      (Rendering|Components|TextRender|SetText (Variables|/Game/MyContent/Blueprints/Lectures/Shield/W_Shield.W_Shield_C|GetDistNum _asw_shield) (Utilities|Text|ToText(Float) _returnvalue_3 "HalfToEven"))
      (Class|Image|SetDesiredSizeOverride (Variables|/Game/MyContent/Blueprints/Lectures/Shield/W_Shield.W_Shield_C|GetShieldBar _asw_shield) (Math|Vector2D|MakeVector2D (* (- 1.0 (/ _returnvalue_3 6.0)) 385.0) 32.0)))))

(event EventBeginPlay)

(event Collision|EventActorBeginOverlap
  (params (OtherActor :type Actor%20Object%20Reference)))

(event EventTick
  (params (DeltaSeconds :type Float%20%28single-precision%29)))

(fn ConstructionScript)