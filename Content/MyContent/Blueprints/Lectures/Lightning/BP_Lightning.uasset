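; BP_Lightning is an actor that repeatedly spawns a lightning effect at its own location.
; On BeginPlay it starts a looping timer that fires every second and a half and spawns the NF_Lightning Niagara system at the root component.
; Each spawned system receives beam width, jitter, and two layers of noise strength and frequency from the Blueprint's variables, passed as float parameters.
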(event Custom|Ef
  (bind _returnvalue (Niagara|SpawnSystematLocation "/Game/MyContent/NiagaraVFX/Lightning/NF_Lightning.NF_Lightning" (Transformation|GetWorldLocation (Variables|Default|GetDefaultSceneRoot))))
  (Niagara|SetNiagaraVariable(Float) _returnvalue "BeamWidthScale" (Variables|Default|GetBWS))
  (Niagara|SetNiagaraVariable(Float) _returnvalue "JitterAmount" (Variables|Default|GetJA))
  (Niagara|SetNiagaraVariable(Float) _returnvalue "NoiseStrength1" (Variables|Default|GetNS1))
  (Niagara|SetNiagaraVariable(Float) _returnvalue "NoiseStrength2" (Variables|Default|GetNS2))
  (Niagara|SetNiagaraVariable(Float) _returnvalue "NoiseFrequency1" (Variables|Default|GetNF1))
  (Niagara|SetNiagaraVariable(Float) _returnvalue "NoiseFrequency2" (Variables|Default|GetNF2)))

(event EventBeginPlay
  (Utilities|Time|SetTimerbyFunctionName 0 "Ef" 1.5 true))

(event Collision|EventActorBeginOverlap
  (params (OtherActor :type Actor%20Object%20Reference)))

(event EventTick
  (params (DeltaSeconds :type Float%20%28single-precision%29)))

(fn ConstructionScript)