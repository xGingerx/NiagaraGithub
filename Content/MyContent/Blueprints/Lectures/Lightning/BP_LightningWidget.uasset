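; BP_LightningWidget is a Lightning lecture actor that shows two widget components while a VR pawn is inside its trigger box.
; On BeginPlay it sets the background colors of the Tekst and Slika elements in the first widget's W_Light, then hides both widgets.
; Box begin and end overlaps toggle their visibility, reacting only when the other actor's class is exactly VRPawn.
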(event OnComponentBeginOverlap(Box)
  (params (OverlappedComponent :type Primitive%20Component%20Object%20Reference) (OtherActor :type Actor%20Object%20Reference) (OtherComp :type Primitive%20Component%20Object%20Reference) (OtherBodyIndex :type Integer) (bFromSweep :type Boolean) (SweepResult :type Hit%20Result%20Structure%20%28by%20ref%29))
  (if (== (Utilities|GetClass OtherActor) "/Game/VRTemplate/Blueprints/VRPawn.VRPawn_C")
    (Rendering|SetVisibility (Variables|Default|GetWidget) true true)))

(event OnComponentEndOverlap(Box)
  (params (OverlappedComponent :type Primitive%20Component%20Object%20Reference) (OtherActor :type Actor%20Object%20Reference) (OtherComp :type Primitive%20Component%20Object%20Reference) (OtherBodyIndex :type Integer))
  (if (== (Utilities|GetClass OtherActor) "/Game/VRTemplate/Blueprints/VRPawn.VRPawn_C")
    (Rendering|SetVisibility (Variables|Default|GetWidget) false false)))

(event EventBeginPlay
  (bind _asw_light (Utilities|Casting|CastToW_Light (UserInterface|GetWidget (Variables|Default|GetWidget))))
  (Class|Button|SetBackgroundColor (Variables|/Game/MyContent/Blueprints/Lectures/Lightning/W_Light.W_Light_C|GetTekst _asw_light) (Utilities|Struct|MakeLinearColor 0.07 0.09 0.36 1.0))
  (Class|Button|SetBackgroundColor (Variables|/Game/MyContent/Blueprints/Lectures/Lightning/W_Light.W_Light_C|GetSlika _asw_light) (Utilities|Struct|MakeLinearColor 0.013 0.0 0.2 0.83))
  (Rendering|SetVisibility (Variables|Default|GetWidget) false false))

(event Collision|EventActorBeginOverlap
  (params (OtherActor :type Actor%20Object%20Reference)))

(event EventTick
  (params (DeltaSeconds :type Float%20%28single-precision%29)))

(fn ConstructionScript)