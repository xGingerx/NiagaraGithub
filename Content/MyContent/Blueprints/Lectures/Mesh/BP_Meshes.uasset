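; BP_Meshes is an actor for the Mesh lecture that shows two widget panels while the VR player is nearby.
; On BeginPlay it hides both panels and tints four elements of the W_Mesh widget, giving Sprite a brighter orange than the dark brown Light, Mesh and Ribbon.
; A Box trigger shows both panels when a VRPawn enters and hides them when it leaves.
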(event OnComponentBeginOverlap(Box)
  (params (OverlappedComponent :type Primitive%20Component%20Object%20Reference) (OtherActor :type Actor%20Object%20Reference) (OtherComp :type Primitive%20Component%20Object%20Reference) (OtherBodyIndex :type Integer) (bFromSweep :type Boolean) (SweepResult :type Hit%20Result%20Structure%20%28by%20ref%29))
  (if (== (Utilities|GetClass OtherActor) "/Game/VRTemplate/Blueprints/VRPawn.VRPawn_C")
    (Rendering|SetVisibility (Variables|Default|GetWidget) true true)))

(event OnComponentEndOverlap(Box)
  (params (OverlappedComponent :type Primitive%20Component%20Object%20Reference) (OtherActor :type Actor%20Object%20Reference) (OtherComp :type Primitive%20Component%20Object%20Reference) (OtherBodyIndex :type Integer))
  (if (== (Utilities|GetClass OtherActor) "/Game/VRTemplate/Blueprints/VRPawn.VRPawn_C")
    (Rendering|SetVisibility (Variables|Default|GetWidget) false false)))

(event EventBeginPlay
  (bind _asw_mesh (Utilities|Casting|CastToW_Mesh (UserInterface|GetWidget (Variables|Default|GetWidget))))
  (Class|Button|SetBackgroundColor (Variables|/Game/MyContent/Blueprints/Lectures/Mesh/W_Mesh.W_Mesh_C|GetLight _asw_mesh) "(R=0.133333,G=0.074510,B=0.000000,A=1.000000)")
  (Class|Button|SetBackgroundColor (Variables|/Game/MyContent/Blueprints/Lectures/Mesh/W_Mesh.W_Mesh_C|GetSprite _asw_mesh) "(R=0.619608,G=0.137255,B=0.000000,A=1.000000)")
  (Rendering|SetVisibility (Variables|Default|GetWidget) false false))

(event Collision|EventActorBeginOverlap
  (params (OtherActor :type Actor%20Object%20Reference)))

(event EventTick
  (params (DeltaSeconds :type Float%20%28single-precision%29)))

(fn ConstructionScript)