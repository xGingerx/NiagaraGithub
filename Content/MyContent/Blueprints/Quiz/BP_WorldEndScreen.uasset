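; World-space end screen for the quiz that shows the player's result through a BP_Quiz_EndScreen widget.
; ShowEndScreen takes the score and maximum, then writes the percentage and a grade from 1 to 5, chosen by fixed ratio thresholds, into the widget's Postotak and Ocjena texts.
; It ends with a check for LectureLevel whose branch does nothing.
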(event Custom|ShowEndScreen
  (params (Score :type Integer) (MaxScore :type Integer))
  (bind _returnvalue (Math|Conversions|ToFloat(Integer) Score))
  (bind _returnvalue_2 (Math|Conversions|ToFloat(Integer) MaxScore))
  (bind _returnvalue_3 (/ _returnvalue _returnvalue_2))
  (bind _asbp_quiz_end_screen (Utilities|Casting|CastToBP_Quiz_EndScreen (UserInterface|GetWidget (Variables|Default|GetWidget))))
  (Rendering|Components|TextRender|SetText (Variables|/Game/MyContent/Blueprints/Quiz/BP_Quiz_EndScreen.BP_Quiz_EndScreen_C|GetPostotak _asbp_quiz_end_screen) (Utilities|Text|ToText(String) (Utilities|String|Append (Utilities|String|ToString(Text) (Utilities|Text|ToText(Float) (* _returnvalue_3 1e+02) "HalfToEven")) " %")))
  (if (< _returnvalue_3 0.5)
    (Rendering|Components|TextRender|SetText (Variables|/Game/MyContent/Blueprints/Quiz/BP_Quiz_EndScreen.BP_Quiz_EndScreen_C|GetOcjena _asbp_quiz_end_screen) "1")
    (elif (< _returnvalue_3 0.6)
      (Rendering|Components|TextRender|SetText (Variables|/Game/MyContent/Blueprints/Quiz/BP_Quiz_EndScreen.BP_Quiz_EndScreen_C|GetOcjena _asbp_quiz_end_screen) "2")
      (elif (< _returnvalue_3 0.75)
        (Rendering|Components|TextRender|SetText (Variables|/Game/MyContent/Blueprints/Quiz/BP_Quiz_EndScreen.BP_Quiz_EndScreen_C|GetOcjena _asbp_quiz_end_screen) "3")
        (elif (< _returnvalue_3 0.9)
          (Rendering|Components|TextRender|SetText (Variables|/Game/MyContent/Blueprints/Quiz/BP_Quiz_EndScreen.BP_Quiz_EndScreen_C|GetOcjena _asbp_quiz_end_screen) "4")
          (else
            (Rendering|Components|TextRender|SetText (Variables|/Game/MyContent/Blueprints/Quiz/BP_Quiz_EndScreen.BP_Quiz_EndScreen_C|GetOcjena _asbp_quiz_end_screen) "5"))))))
  (bind _returnvalue_4 (Game|GetCurrentLevelName true))
  (if (Utilities|Enum|Equal(Enum) _returnvalue_4 "LectureLevel")
    _))

(fn ConstructionScript)