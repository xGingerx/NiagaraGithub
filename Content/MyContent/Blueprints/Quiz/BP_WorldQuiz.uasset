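; World-placed quiz actor that runs a list of questions through a BP_QuizTemplate widget and tallies correct answers.
; StartQuiz gathers the four answer buttons, darkens question text in LectureLevel, and calls NextQuestion.
; NextQuestion increments the passed-in score on correct answers and feeds the next question to the widget.
; When questions run out, it spawns BP_WorldEndScreen at a hardcoded level-dependent transform, shows the score, and destroys itself.
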(event Custom|StartQuiz
  ;[1 1 1] Initialize quiz (buttons for answers) and start displaying questions
  (bind _asbp_quiz_template (Utilities|Casting|CastToBP_QuizTemplate (UserInterface|GetWidget (Variables|Default|GetWidget))))
  (Variables|/Game/MyContent/Blueprints/Quiz/BP_QuizTemplate.BP_QuizTemplate_C|SetA1_Var _asbp_quiz_template (Utilities|Array|MakeArray (Variables|/Game/MyContent/Blueprints/Quiz/BP_QuizTemplate.BP_QuizTemplate_C|Geta1 _asbp_quiz_template) (Variables|/Game/MyContent/Blueprints/Quiz/BP_QuizTemplate.BP_QuizTemplate_C|Geta2 _asbp_quiz_template) (Variables|/Game/MyContent/Blueprints/Quiz/BP_QuizTemplate.BP_QuizTemplate_C|Geta3 _asbp_quiz_template) (Variables|/Game/MyContent/Blueprints/Quiz/BP_QuizTemplate.BP_QuizTemplate_C|Geta4 _asbp_quiz_template)))
  (bind _returnvalue (Game|GetCurrentLevelName true))
  (if (Utilities|Enum|Equal(Enum) _returnvalue "LectureLevel")
    (Appearance|SetColorandOpacity (Variables|/Game/MyContent/Blueprints/Quiz/BP_QuizTemplate.BP_QuizTemplate_C|GetQuestion _asbp_quiz_template) (Utilities|Struct|MakeSlateColor "(R=0.000000,G=0.000000,B=0.000000,A=1.000000)") :!class /Script/UMG.TextBlock))
  (CallFunction|NextQuestion false))

(event Collision|EventActorBeginOverlap
  (params (OtherActor :type Actor%20Object%20Reference)))

(event EventTick
  (params (DeltaSeconds :type Float%20%28single-precision%29)))

(event EventNextQuestion
  (params (CorrectAnswer :type Boolean) (Score :type Integer))
  (bind _currentquestion (Variables|Default|GetCurrentQuestion))
  (bind _questions (Variables|Default|GetQuestions))
  (bind _returnvalue (Utilities|Array|LastIndex _questions))
  (bind _returnvalue_2 (+ _returnvalue 1))
  (if CorrectAnswer
    (Math|Integer|IncrementInt (Variables|Default|GetScore)
      (:%20%20
        _)))
  (if (>= _returnvalue (Variables|Default|GetCurrentQuestion))
    ;[1 1 1] If there is more questions
    (bind _asbp_quiz_template (Utilities|Casting|CastToBP_QuizTemplate (UserInterface|GetWidget (Variables|Default|GetWidget))))
    (Default|InitializeQuiz _asbp_quiz_template (Utilities|Array|Get(acopy) (Variables|Default|GetQuestions) _currentquestion))
    (Math|Integer|IncrementInt _currentquestion)
    (else
      (bind _returnvalue_3 (Game|GetCurrentLevelName true))
      (if (Utilities|Enum|Equal(Enum) _returnvalue_3 "LectureLevel")
        (bind _returnvalue_4 (Game|SpawnActorfromClass "/Game/MyContent/Blueprints/Quiz/BP_WorldEndScreen.BP_WorldEndScreen_C" (Math|Transform|MakeTransform "1015.000000,-865.000000,-508.000000" "0.000000,90.000000,0.000000") "Undefined" 0 0))
        (Default|ShowEndScreen _returnvalue_4 Score _returnvalue_2)
        (Actor|DestroyActor)
        (else
          (bind _returnvalue_5 (Game|SpawnActorfromClass "/Game/MyContent/Blueprints/Quiz/BP_WorldEndScreen.BP_WorldEndScreen_C" (Math|Transform|MakeTransform "1937.000000,-405.000000,339.000000" "0.000000,90.000000,0.000000") "Undefined" 0 0))
          (Default|ShowEndScreen _returnvalue_5 Score _returnvalue_2)
          (Actor|DestroyActor))))))

(fn ConstructionScript)